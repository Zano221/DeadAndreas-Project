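; Health pickup that heals a player on overlap, only when their health is below its default.
; On BeginPlay it writes the rounded-up heal amount into a widget that stays hidden by being visible in scene capture only.
; A successful pickup swaps the flipbook, reveals and eases the widget upward with a click sound, then destroys the actor after a short delay.
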(event `self.ReceiveBeginPlay`
  (`parent.ReceiveBeginPlay`)
  (`PrimitiveComponent.SetVisibleInSceneCaptureOnly` (`self.HealthPickWidget`) true)
  (bind _aswbp_health_pick (cast `/Game/Blueprints/UI/WBP_HealthPick` (`WidgetComponent.GetWidget` (`self.HealthPickWidget`))))
  (bind _output_get (set `self.WBP_ValueRef` _aswbp_health_pick))
  (`/Game/Blueprints/UI/WBP_HealthPick.UpdateHealthPickValue` _output_get (`KismetMathLibrary.Conv_Int64ToInt` (`KismetMathLibrary.FCeil64` (`self.HealthValue`)))))

(event `self.InteractiveCollider.OnComponentBeginOverlap`
  (params (OverlappedComponent :type "PrimitiveComponent Object Reference") (OtherActor :type "Actor Object Reference") (OtherComp :type "PrimitiveComponent Object Reference") (OtherBodyIndex :type Integer) (bFromSweep :type Boolean) (SweepResult :type "HitResult Structure (by ref)"))
  (bind _asbp_player_base (cast `/Game/Blueprints/BP_PlayerBase` OtherActor))
  (`self.Interact` _asbp_player_base))

(event `PostHealthPick`
  (bind _healthpickwidget (`self.HealthPickWidget`))
  (`|ExecutionSequence`
    (:`then_0`
      (`PrimitiveComponent.SetVisibleInSceneCaptureOnly` (`self.HealthPickWidget`) false)
      (`KismetSystemLibrary.MoveComponentTo` _healthpickwidget (0.0 0.0 240.0) (`SceneComponent.RelativeRotation` _healthpickwidget) true false 0.8))
    (:`then_1`
      (`GameplayStatics.PlaySound2D` "/Engine/VREditor/Sounds/UI/Click_on_Button_Cue.Click_on_Button_Cue" 1.0 1.0 0.0 null null)
      (`KismetSystemLibrary.Delay` 0.8)
      (`self.K2_DestroyActor`))))

(fn `Interact`
  (params (PlayerRef :type "/Game/Blueprints/BP_PlayerBase Object Reference"))
  (if (< (`/Game/Blueprints/BP_PlayerBase.Health` PlayerRef) (`/Game/Blueprints/BP_PlayerBase.DefaultHealth` PlayerRef))
    (`/Game/Blueprints/BP_PlayerBase.AddHealth` PlayerRef (`self.HealthValue`))
    (`PaperFlipbookComponent.SetFlipbook` (`self.PaperFlipbook`) "/Game/Assets/Flipbooks/Lol_Moving.Lol_Moving")
    (`self.PostHealthPick`)))

(fn `UserConstructionScript`
  (`parent.UserConstructionScript`))