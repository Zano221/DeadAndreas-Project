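; BP_InteractiveGameEnd is an interactive trigger that ends the game in a win when the player reaches it.
; Overlap on its InteractiveCollider casts the other actor to BP_PlayerBase and passes it to Interact.
; Interact sets the player's GameFinished flag, disables their input, and adds a WBP_GameWin widget to the viewport.
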(event `self.ReceiveBeginPlay`
  (`parent.ReceiveBeginPlay`))

(event `self.InteractiveCollider.OnComponentBeginOverlap`
  (params (OverlappedComponent :type "PrimitiveComponent Object Reference") (OtherActor :type "Actor Object Reference") (OtherComp :type "PrimitiveComponent Object Reference") (OtherBodyIndex :type Integer) (bFromSweep :type Boolean) (SweepResult :type "HitResult Structure (by ref)"))
  (bind _asbp_player_base (cast `/Game/Blueprints/BP_PlayerBase` OtherActor))
  (`self.Interact` _asbp_player_base))

(fn `Interact`
  (params (PlayerRef :type "/Game/Blueprints/BP_PlayerBase Object Reference"))
  (set `/Game/Blueprints/BP_PlayerBase.GameFinished` true PlayerRef)
  (`self.DisableInput` PlayerRef null)
  (bind _returnvalue (`|CreateWidget` "/Game/Blueprints/UI/WBP_GameWin.WBP_GameWin_C"))
  (`UserWidget.AddToViewport` _returnvalue 0))

(fn `UserConstructionScript`
  (`parent.UserConstructionScript`))