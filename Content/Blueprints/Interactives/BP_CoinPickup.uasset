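; Coin pickup interactive with a looping flipbook that awards the player a fixed score when interacted with.
; BeginPlay writes the value into its WBP_MoneyReward widget, which construction hides by making it visible in scene capture only.
; Interact updates the player's score, clears the flipbook, calls the parent, then fires PostCoinCollected.
; That event reveals and floats the widget upward with a sound, destroying the actor after a delay kept in the EventGraph.
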(event `self.ReceiveBeginPlay`
  (set `self.ScorePoints` 50)
  (`PaperFlipbookComponent.SetLooping` (`self.PaperFlipbook`) true)
  (bind _aswbp_money_reward (cast `/Game/Blueprints/UI/WBP_MoneyReward` (`WidgetComponent.GetWidget` (`self.WidgetScore`))))
  (bind _output_get (set `self.WBP_ValueRef` _aswbp_money_reward))
  (`/Game/Blueprints/UI/WBP_MoneyReward.UpdateScore` _output_get (`self.ScorePoints`)))

(event `PostCoinCollected`
  (bind _widgetscore (`self.WidgetScore`))
  ;[1 1 1] Executes the Widget animation after collision, it's here because "Delay" can only be used here
  (`|ExecutionSequence`
    (:`then_0`
      (`PrimitiveComponent.SetVisibleInSceneCaptureOnly` (`self.WidgetScore`) false)
      (`KismetSystemLibrary.MoveComponentTo` _widgetscore (0.0 0.0 240.0) (`SceneComponent.RelativeRotation` _widgetscore) true false 0.8))
    (:`then_1`
      (`GameplayStatics.PlaySound2D` "/Engine/VREditor/Sounds/UI/Click_on_Button_Cue.Click_on_Button_Cue" 1.0 1.0 0.0 null null)
      (`KismetSystemLibrary.Delay` 0.8)
      (`self.K2_DestroyActor`))))

(fn `Interact`
  (params (PlayerRef :type "/Game/Blueprints/BP_PlayerBase Object Reference"))
  (`/Game/Blueprints/BP_PlayerBase.UpdateScore` PlayerRef (`self.ScorePoints`))
  (`PaperFlipbookComponent.SetFlipbook` (`self.PaperFlipbook`) null)
  (`parent.Interact` null)
  (`self.PostCoinCollected`))

(fn `UserConstructionScript`
  (`PrimitiveComponent.SetVisibleInSceneCaptureOnly` (`self.WidgetScore`) true)
  (`parent.UserConstructionScript`))